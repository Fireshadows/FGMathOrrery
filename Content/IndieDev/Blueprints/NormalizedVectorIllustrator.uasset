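; Editor illustrator Blueprint that visualizes how a relative offset vector normalizes into a direction.
; The construction script places Target at Offset, then NormalVizualiser prints the raw and normalized vectors and aims an Arrow along that direction.
; An optionally visible Projection component sits at the normalized vector scaled by Distance, with a text label showing that distance.
; A grid-snapping step for Offset exists but is disconnected.
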(fn `NormalVizualiser`
  (bind _distance (`self.Distance`))
  (bind _relativelocation (`SceneComponent.RelativeLocation` (`self.Target`)))
  (bind _returnvalue (`KismetMathLibrary.Normal` _relativelocation))
  (`TextRenderComponent.K2_SetText` (`self.TextRender`) (`KismetTextLibrary.Conv_StringToText` (`KismetStringLibrary.Concat_StrStr` "Real Offset \n" (`KismetStringLibrary.Conv_VectorToString` _relativelocation) " \n \nNormalized Vector \n" (`KismetStringLibrary.Conv_VectorToString` _returnvalue))))
  (`SceneComponent.K2_SetRelativeRotation` (`self.Arrow`) (`KismetMathLibrary.Conv_VectorToRotator` _returnvalue) false false)
  (`SceneComponent.K2_SetRelativeLocation` (`self.Projection`) (* _returnvalue _distance) false false)
  (`TextRenderComponent.K2_SetText` (`self.Projection Text`) (`KismetTextLibrary.Conv_StringToText` (`KismetStringLibrary.Concat_StrStr` "Projection \n" (`KismetStringLibrary.Conv_DoubleToString` _distance) " \nDistance")))
  (`SceneComponent.SetVisibility` (`self.Projection`) (`self.Show Projection`) true))

(fn `UserConstructionScript`
  (`SceneComponent.K2_SetRelativeLocation` (`self.Target`) (`self.Offset`) false false)
  (`self.NormalVizualiser`))